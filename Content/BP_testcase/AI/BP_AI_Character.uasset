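; Test AI character that moves toward the player on BeginPlay, prints messages, then roams between preset points.
; After a short delay, a looping timer fires Walking, which sends it to a random PointsToMove actor.
; Both AI moves continue on request and again on success, and the random index can overrun the array.
; RandLocation returns the first point differing from LastLocation but is never called here.
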(event Custom|Walking
  (bind _pointstomove (Variables|routine|GetPointsToMove))
  (AI|AIMoveTo self "0, 0, 0" (Utilities|Array|Get(acopy) _pointstomove (Math|Random|RandomIntegerinRange 0 (Utilities|Array|Length _pointstomove))) 5.0 false
    (:then
      _)
    (:OnSuccess
      _))
  (Development|PrintString "Nothing"))

(event EventBeginPlay
  (AI|AIMoveTo self "0, 0, 0" (Game|GetPlayerCharacter 0) 5.0 false
    (:then
      _)
    (:OnSuccess
      _))
  (Development|PrintString "Got you")
  (Utilities|FlowControl|Delay 3.0)
  (Development|PrintString "Let me walk around")
  (Utilities|Time|SetTimerbyEvent (delegate Custom|Walking) 3.0 true)
  (Development|PrintString "hmmm"))

(event Collision|EventActorBeginOverlap
  (params (OtherActor :type Actor%20Object%20Reference)))

(event EventTick
  (params (DeltaSeconds :type Float%20%28single-precision%29)))

(fn ConstructionScript)

(fn RandLocation
  (for _array_element (Variables|routine|GetPointsToMove)
    (if (not (Utilities|Operators|EqualEqual (Variables|Default|GetLastLocation) (Transformation|GetActorLocation _array_element) 0.0))
      (return (Transformation|GetActorLocation _array_element)))))