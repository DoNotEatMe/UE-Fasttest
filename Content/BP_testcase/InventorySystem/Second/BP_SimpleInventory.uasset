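; BP_SimpleInventory is a simple stacking inventory that picks up BP_ExampleLoot objects.
; LootAndDestroy passes the other actor to ClaimLoot, then destroys the returned loot actor.
; ClaimLoot casts to the loot class and merges its name and count into the Items array.
; A matching name increases that entry's count; an empty array or no match appends a new entry.
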(event Custom|LootAndDestroy
  (params (Other%20Actor :type Actor%20Object%20Reference))
  (bind _loot_object (CallFunction|ClaimLoot Other%20Actor))
  (Actor|DestroyActor _loot_object))

(event EventBeginPlay)

(event EventTick
  (params (DeltaSeconds :type Float%20%28single-precision%29)))

(fn ClaimLoot
  (params (LootObject :type Object%20Object%20Reference))
  (bind _asbp_example_loot (Utilities|Casting|CastToBP_ExampleLoot LootObject))
  (bind _output_get (LocalVariables|SetLocal_LootObject _asbp_example_loot))
  (LocalVariables|SetLocal_InputName (.Name (Utilities|Struct|BreakF_ItemStruct_Second (Variables|/Game/BP_testcase/Items/Second/BP_ExampleLoot.BP_ExampleLoot_C|GetItemSetup _output_get))))
  (LocalVariables|SetLocal_InputCount (.Count (Utilities|Struct|BreakF_ItemStruct_Second (Variables|/Game/BP_testcase/Items/Second/BP_ExampleLoot.BP_ExampleLoot_C|GetItemSetup _output_get))))
  ;[1 1 1] if empty adding elem without checks
  (if (Utilities|Array|IsEmpty (Variables|Default|GetItems))
    (Utilities|Array|Add (Variables|Default|GetItems) (Variables|/Game/BP_testcase/Items/Second/BP_ExampleLoot.BP_ExampleLoot_C|GetItemSetup (LocalVariables|GetLocal_LootObject)))
    (return (LocalVariables|GetLocal_LootObject))
    (else
      ;[1 1 1] If not empty checking same names ? Count+count : Add elem
      (for (_array_element _array_index) (Variables|Default|GetItems)
        (if (Utilities|Enum|Equal(Enum) (.name _array_element) (LocalVariables|GetLocal_InputName))
          (Utilities|Array|SetArrayElem (Variables|Default|GetItems) _array_index (Utilities|Struct|MakeF_ItemStruct_Second (.name _array_element) (+ (.count _array_element) (LocalVariables|GetLocal_InputCount))))
          (return (LocalVariables|GetLocal_LootObject))
          (elif (not (!= _array_index (Utilities|Array|LastIndex (Variables|Default|GetItems))))
            (Utilities|Array|Add (Variables|Default|GetItems) (Utilities|Struct|MakeF_ItemStruct_Second (LocalVariables|GetLocal_InputName) (LocalVariables|GetLocal_InputCount)))
            (return (LocalVariables|GetLocal_LootObject))))))))